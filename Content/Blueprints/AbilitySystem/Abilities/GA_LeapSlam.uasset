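; Leap slam Gameplay Ability that launches the player character to a nearby valid point, then damages and knocks back targets on landing.
; After range checks and commit, it disables movement, rotates toward the target, pauses briefly, then runs a curve-driven Leap task.
; Landing starts targeting, whose data feeds the damage effect and radial knockback.
; Pawn collision is ignored from leap start until shortly after impact to avoid position snapping.
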(event Ability|EventActivateAbility
  (bind _ascharacter (Utilities|Casting|CastToCharacter (Ability|GetAvatarActorfromActorInfo)))
  (Variables|References|SetCharacter _ascharacter)
  (bind _asplayer_controller (Utilities|Casting|CastToPlayerController (Pawn|GetController _ascharacter)))
  (Variables|References|SetPlayerController _asplayer_controller)
  ;[0.15 0.15 0.15 0.5] Calculate where to leap
  (bind _returnvalue (Class|GASTargetingLibrary|CalculateLeapTarget (Ability|GetAvatarActorfromActorInfo) (Variables|References|GetPlayerController) (Transformation|GetActorLocation (Ability|GetAvatarActorfromActorInfo)) 4e+02 5e+02))
  ;[0.15 0.15 0.15 0.5] Check if we can leap to location
  (if (.bisvalid _returnvalue)
    (bind _output_get (Variables|Default|SetLeapTargetLocation (.location _returnvalue)))
    (if (>= (Math|Vector|Distance(Vector) _output_get (Transformation|GetActorLocation (Ability|GetAvatarActorfromActorInfo))) 2e+02)
      ;[0.15 0.15 0.15 0.5] If so, then we can commit this ability.
      (bind _returnvalue_2 (Ability|CommitAbility))
      (if _returnvalue_2
        ;[0.15 0.15 0.15 0.5] Avoid player trying to move during leap
        (Pawn|Components|CharacterMovement|DisableMovement (Variables|/Script/Engine.Character|GetCharacterMovement (Variables|References|GetCharacter)))
        ;[0.15 0.15 0.15 0.5] Simple rotation towards the leap location. For a more polished version, we could do a pivot animation
        (|RotateCharactertoLocation (Variables|Default|GetLeapTargetLocation) 8.0
          (:then
            ;[0.15 0.15 0.15 0.5] Game feel: This can work as an "anticipation" to leap
            (Utilities|FlowControl|Delay 0.1)
            ;[0.15 0.15 0.15 0.5] Leap to target. Once finish, target in AoE.
            ;
            ; The events can be used to integrate animations. Here we have:
            ; 1. Leap started
            ; 2. Leap apex
            ; 3. Leap landed
            ;
            ; How I would implement:
            ;
            ; Having three animations: LeapingLoop, LeapTransition (Raising->Falling), LeapFalling
            ; 1. Start Leaping Loop on exec output.
            ; 2. During apex, use leap transition aniomation and then start leap falling animation
            ;
            ; This would be easy using an AnimBP state machine
            (|Leap (Variables|Default|GetLeapTargetLocation) "/Game/LeapPrototype/FC_Leap_HorizontalAcceleration.FC_Leap_HorizontalAcceleration" "/Game/LeapPrototype/FC_Leap_HeightCurve.FC_Leap_HeightCurve" 1.0 4e+02
              (:then
                (Collision|SetCollisionResponsetoChannel (Variables|/Script/Engine.Character|GetCapsuleComponent (Variables|References|GetCharacter)) "ECC_Pawn" "ECR_Ignore"))
              (:OnLanded
                (Class|GameplayAbilityLeapSlam|StartTargeting false)))))
        (else
          (Ability|EndAbility)))
      (else
        (Ability|EndAbility)))
    (else
      (Ability|EndAbility))))

(event EventOnTargetDataReady
  (params (TargetData :type Gameplay%20Ability%20Target%20Data%20Handle%20Structure%20%28by%20ref%29))
  ;[0.15 0.15 0.15 0.5] Apply damage to targets
  (GameplayEffects|ApplyGameplayEffectToTarget TargetData "/Game/Blueprints/AbilitySystem/GameplayEffects/GE_ApplyDamage.GE_ApplyDamage_C" 1 1)
  ;[0.15 0.15 0.15 0.5] Apply radial knockback according to designer-defined distance
  (Class|TDWTestGameplayAbility|ApplyRadialKnockbacktoCharacters (Variables|References|GetCharacter) (Ability|TargetData|GetActorsfromTargetData TargetData) 1.6e+02 3e+02 1.0)
  ;[0.15 0.15 0.15 0.5] Wait a bit to re-enable collision, to avoid position snap due to physics resolve. We should be fine here, as cooldown will always be greater then 0.4s
  (Utilities|FlowControl|Delay 0.4)
  (Collision|SetCollisionResponsetoChannel (Variables|/Script/Engine.Character|GetCapsuleComponent (Variables|References|GetCharacter)) "ECC_Pawn" "ECR_Block")
  (Ability|EndAbility))

(fn ApplyKnockbacktoTargets
  (params (TargetData :type Gameplay%20Ability%20Target%20Data%20Handle%20Structure%20%28by%20ref%29))
  (for _array_element (Ability|TargetData|GetActorsfromTargetData TargetData)
    (if (<= (Math|Vector|Distance(Vector) (Transformation|GetActorLocation _array_element) (Transformation|GetActorLocation (Variables|References|GetCharacter))) 1.6e+02)
      (bind _ascharacter (Utilities|Casting|CastToCharacter _array_element))
      (Class|CombatStaticsLibrary|ApplyRadialKnockback (Variables|References|GetCharacter) _ascharacter 3e+02 1.0))))